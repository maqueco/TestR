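; Obstacle spawner actor that scatters cubes, spheres and life objects at random points inside its Box volume.
; Tick calls the Spawner event every frame, which loops over ItemCount with a SpawnDelay Delay inside the loop body.
; Cascading range checks, each on a fresh random roll, choose cube, sphere, life or nothing.
; Each spawn function adds a Child Actor Component at a random point from the Box's relative location and extent.
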(event `self.ReceiveBeginPlay`)

(event `self.ReceiveTick`
  (params (DeltaSeconds :type "Float (single-precision)"))
  (`self.Spawner`))

(event `Spawner`
  (bind _returnvalue (`KismetMathLibrary.RandomFloatInRange` 0.0 1.0))
  (for _ (range (+ (`self.ItemCount`) 1))
    (`KismetSystemLibrary.Delay` (`self.SpawnDelay`))
    (if (`KismetMathLibrary.InRange_FloatFloat` _returnvalue 0.0 0.3)
      (`self.Spawn Cube`)
      (elif (`KismetMathLibrary.InRange_FloatFloat` _returnvalue 0.4 0.7)
        (`self.Spawn Sphere`)
        (elif (`KismetMathLibrary.InRange_FloatFloat` _returnvalue 0.8 1.0)
          (`self.Spawn Life`))))))

(fn `Spawn Cube`
  (bind _box (`self.Box`))
  (`AddComponent|NODE_AddChildActorComponent-0` :`RelativeTransform` (`KismetMathLibrary.Conv_VectorToTransform` (`KismetMathLibrary.RandomPointInBoundingBox` (`SceneComponent.RelativeLocation` _box) (`BoxComponent.BoxExtent` _box)))))

(fn `Spawn Life`
  (bind _box (`self.Box`))
  (`AddComponent|NODE_AddChildActorComponent-3` :`RelativeTransform` (`KismetMathLibrary.Conv_VectorToTransform` (`KismetMathLibrary.RandomPointInBoundingBox` (`SceneComponent.RelativeLocation` _box) (`BoxComponent.BoxExtent` _box)))))

(fn `Spawn Sphere`
  (bind _box (`self.Box`))
  (`AddComponent|NODE_AddChildActorComponent-4` :`RelativeTransform` (`KismetMathLibrary.Conv_VectorToTransform` (`KismetMathLibrary.RandomPointInBoundingBox` (`SceneComponent.RelativeLocation` _box) (`BoxComponent.BoxExtent` _box)))))

(fn `UserConstructionScript`)